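; BP_Base_Object is an interactable base object that can switch off linked objects acting as walls.
; Interact broadcasts its LinkingID to every other BP_Base_Object, then plays an optional sound.
; Objects with a matching ID hide their sprites and disable collision via WallOff; WallOn is not called here.
; GetNextDialog picks random or cycling lines, but its text box hookup is disconnected from any event.
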(event `/Game/Base_Items/BPI_Interact.Interact`
  (`|ExecutionSequence`
    (:`then_0`
      (`KismetSystemLibrary.PrintText` "Interact_Initiated" true true (struct :`G` 0.838155 :`B` 1.0 :`A` 1.0)))
    (:`then_1`
      (`self.Send_Signal_To_Walls`))
    (:`then_2`
      (`self.Play_Sound`))))

(fn `Get_Next_Dialog`
  (returns (Out_text :type String))
  (bind _outitem (`KismetArrayLibrary.Array_Random` (`self.Dialog_Text`)))
  (if (`self.Is_Dialog_Lines_Random`)
    (`|ExecutionSequence`
      (:`then_0`
        (`KismetSystemLibrary.PrintString` _outitem))
      (:`then_1`
        (return _outitem)))
    (else
      ; Check block
      (if (>= (`self.Current_Dialog_Line`) (`KismetArrayLibrary.Array_Length` (`self.Dialog_Text`)))
        (set `self.Current_Dialog_Line` 0))
      (`|ExecutionSequence`
        (:`then_0`
          (set `self.Temp_text` (`|GetArrayItem` (`self.Dialog_Text`) (`self.Current_Dialog_Line`))))
        (:`then_1`
          ; Increment block
          (bind _result (`/Engine/EditorBlueprintResources/StandardMacros.IncrementInt` (`self.Current_Dialog_Line`))
            (:`  `
              (set `self.Current_Dialog_Line` _result)
              (`|ExecutionSequence`
                (:`then_0`
                  (`KismetSystemLibrary.PrintString` (`self.Temp_text`)))
                (:`then_1`
                  (return (`self.Temp_text`)))))))))))

(fn `Play_Sound`
  (if (!= (`self.InteractSound`) null)
    (`GameplayStatics.PlaySoundAtLocation` (`self.InteractSound`) (`self.K2_GetActorLocation`) (struct) 1.0 1.0 0.0 null null null null)))

(fn `Receive_Signal_As_Wall`
  (params (Received_Signal_ID :type String))
  (`|ExecutionSequence`
    (:`then_0`
      (`KismetSystemLibrary.PrintText` "Received_Signal"))
    (:`then_1`
      (if (`KismetStringLibrary.EqualEqual_StrStr` Received_Signal_ID (`self.Linking_ID`))
        (`self.Wall_Off`)))))

(fn `Send_Signal_To_Walls`
  (bind _outactors (`GameplayStatics.GetAllActorsOfClass` "BP_Base_Object_C"))
  (for _array_element _outactors
    (if (!= _array_element self)
      (`self.Receive_Signal_As_Wall` _array_element (`self.Linking_ID`)))))

(fn `UserConstructionScript`)

(fn `Wall_Off`
  (`SceneComponent.SetVisibility` (`self.2D_Sprite`) false false)
  (`SceneComponent.SetVisibility` (`self.2D_Billboard`) false false)
  (`SceneComponent.SetVisibility` (`self.Box_Collision`) false false)
  (`PrimitiveComponent.SetCollisionEnabled` (`self.Box_Collision`) "NoCollision")
  (`PrimitiveComponent.SetCollisionEnabled` (`self.2D_Sprite`) "NoCollision")
  (`PrimitiveComponent.SetCollisionEnabled` (`self.2D_Billboard`) "NoCollision")
  (`KismetSystemLibrary.PrintString` "Wall_Off" true true (struct :`R` 0.033814 :`G` 1.0 :`A` 1.0)))

(fn `Wall_On`
  (`SceneComponent.SetVisibility` (`self.2D_Sprite`) true false)
  (`SceneComponent.SetVisibility` (`self.2D_Billboard`) true false)
  (`PrimitiveComponent.SetCollisionEnabled` (`self.Box_Collision`) "QueryAndPhysics")
  (`KismetSystemLibrary.PrintString` "Wall_On" true true (struct :`R` 0.033814 :`G` 1.0 :`A` 1.0)))