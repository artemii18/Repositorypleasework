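; BP_Wall is a test wall actor that can be switched off by a signal and restored with a debug key.
; ReceiveSignal compares the incoming ID with AnomalyID and, on a match, disables CollisionBox collision and hides the Plane and its children.
; Pressing or releasing the 0 key restores collision and shows the Plane without propagating to children.
; Both state changes print debug text.
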(event `Key|Zero` :consume false
  (params (Key :type "Key Structure"))
  (:`Pressed`
    (`self.Set_Enabled_True` :!label _label))
  (:`Released`
    (goto _label)))

(fn `Receive_Signal`
  (params (Incoming_ID :type String))
  (if (`KismetStringLibrary.EqualEqual_StrStr` Incoming_ID (`self.Anomaly_ID`))
    (`self.Set_Enabled_False`)))

(fn `Set_Enabled_False`
  (`PrimitiveComponent.SetCollisionEnabled` (`self.CollisionBox`) "NoCollision")
  (`SceneComponent.SetVisibility` (`self.Plane`) false true)
  (`KismetSystemLibrary.PrintText` "Wall_Active_FALSE"))

(fn `Set_Enabled_True`
  (`PrimitiveComponent.SetCollisionEnabled` (`self.CollisionBox`) "QueryAndPhysics")
  (`SceneComponent.SetVisibility` (`self.Plane`) true false)
  (`KismetSystemLibrary.PrintText` "Wall_Active_TRUE"))

(fn `UserConstructionScript`)